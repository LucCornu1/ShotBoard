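; Test pawn for a physics-driven snowboard, steered by Forward and Right input axes.
; Forward pushes the board along the actor's forward vector, while Right applies opposite local forces at both ends to turn it.
; Each tick, a short downward trace detects ground; on a hit, velocity is redirected along the actor's right vector at the same speed and spin is clamped.
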(event `self.ReceiveBeginPlay`
  (`self.K2_SetActorRotation` (struct :`Yaw` -90.0)))

(event `self.ReceiveTick`
  (params (DeltaSeconds :type "Float (single-precision)"))
  (bind (_outhit _returnvalue) (`KismetSystemLibrary.LineTraceSingle` :`Start` (`self.K2_GetActorLocation`) :`End` (`KismetMathLibrary.TransformLocation` (`self.GetTransform`) (0.0 0.0 -10.0)) :`TraceChannel` "TraceTypeQuery1" :`DrawDebugType` "ForOneFrame"))
  (if _returnvalue
    (bind _returnvalue_2 (`PrimitiveComponent.GetPhysicsLinearVelocity` (`self.Snowboard`) "None"))
    (`PrimitiveComponent.SetPhysicsLinearVelocity` (`self.Snowboard`) (* (`self.GetActorRightVector`) (`KismetMathLibrary.VSize` _returnvalue_2)) false "None")
    (`PrimitiveComponent.SetPhysicsAngularVelocityInDegrees` (`self.Snowboard`) (`KismetMathLibrary.ClampVectorSize` (`PrimitiveComponent.GetPhysicsAngularVelocityInDegrees` (`self.Snowboard`) "None") -50.0 50.0) false "None")
    (set `self.AngularVelocity` (`PrimitiveComponent.GetPhysicsAngularVelocityInDegrees` (`self.Snowboard`) "None"))))

(event `InputAxis|Forward`
  (params (AxisValue :type "Float (single-precision)"))
  (set `self.Velocity` (* (`self.GetActorForwardVector`) (* AxisValue 1000.0)))
  (`PrimitiveComponent.AddForce` (`self.Snowboard`) (`self.Velocity`) "None" false))

(event `InputAxis|Right`
  (params (AxisValue :type "Float (single-precision)"))
  (bind _returnvalue (* AxisValue 10.0))
  (bind _snowboard (`self.Snowboard`))
  (if true
    (`PrimitiveComponent.AddForceAtLocationLocal` _snowboard (`KismetMathLibrary.MakeVector` 0.0 _returnvalue) (50.0 0.0 0.0) "None")
    (`PrimitiveComponent.AddForceAtLocationLocal` _snowboard (`KismetMathLibrary.MakeVector` 0.0 (* -1 _returnvalue)) (-50.0 0.0 0.0) "None")))

(fn `UserConstructionScript`)