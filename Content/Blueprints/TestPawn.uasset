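; TestPawn is an experimental physics movement pawn whose Tick, Forward and Right input events currently have no effect.
; Its disconnected node groups hold trial approaches: torque, local rotation, forward force, and opposed offset forces for turning.
; Other unused fragments sketch a short downward trace and a velocity correction that realigns speed to the forward vector and clamps angular velocity.
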(event `self.ReceiveTick`
  (params (DeltaSeconds :type "Float (single-precision)")))

(event `InputAxis|Forward`
  (params (AxisValue :type "Float (single-precision)")))

(event `InputAxis|Right`
  (params (AxisValue :type "Float (single-precision)"))
  (if true
    _))

(fn `UserConstructionScript`)